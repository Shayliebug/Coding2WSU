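; SingletonBP is a game-instance manager that saves, loads and deletes per-level records of collected coins, using the level name as slot name.
; Load waits briefly, clears AlreadyCollectedObjects, then destroys the actors listed in the slot's SG_Objects PickedUpCoins.
; Save reuses or creates that save object and overwrites its list with AlreadyCollectedObjects, which Load never refills from the save.
; DeleteSave removes the current level's slot.
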(event Custom|Load
  (Utilities|FlowControl|Delay 0.2)
  (bind _returnvalue (Game|GetCurrentLevelName true))
  (Utilities|Array|Clear (Variables|Default|GetAlreadyCollectedObjects)) ; New Level clear out this playthru's array of collected objects
  ;[0 0.4171 1] LoadGame
  (Development|PrintString (Utilities|String|Append "Starting load in level" _returnvalue ", wish me luck"))
  (bind _returnvalue_2 (SaveGame|DoesSaveGameExist _returnvalue))
  (if _returnvalue_2
    (bind _returnvalue_3 (SaveGame|LoadGamefromSlot _returnvalue))
    (bind _assg_objects (Utilities|Casting|CastToSG_Objects _returnvalue_3))
    (Variables|Default|SetAs%20SG%20Objects _assg_objects) ; reference to save game 'object'
    (for _array_element (Variables|/Game/SG_Objects.SG_Objects_C|GetPickedUpCoins _assg_objects)
      (Actor|DestroyActor _array_element))))

(event Custom|DeleteSave
  (Development|PrintString "Starting DeleteSave")
  (bind _returnvalue (Game|GetCurrentLevelName true))
  (bind _returnvalue_2 (SaveGame|DoesSaveGameExist _returnvalue))
  (if _returnvalue_2
    (SaveGame|DeleteGameinSlot _returnvalue)
    (Development|PrintString "Save Deleted!")
    (else
      (Development|PrintString "No Save Game Exists!"))))

(event Custom|Save
  (Development|PrintString "Starting Save")
  (bind _returnvalue (Game|GetCurrentLevelName true))
  (bind _returnvalue_2 (SaveGame|DoesSaveGameExist _returnvalue))
  (if _returnvalue_2
    (bind _returnvalue_3 (SaveGame|LoadGamefromSlot _returnvalue))
    (Variables|Default|SetSaver%20Subclass _returnvalue_3)
    (else
      (bind _returnvalue_4 (SaveGame|CreateSaveGameObject "/Game/SG_Objects.SG_Objects_C"))
      (Variables|Default|SetSaver%20Subclass _returnvalue_4)))
  (bind _assg_objects (Utilities|Casting|CastToSG_Objects (Variables|Default|GetSaver%20Subclass)))
  (Variables|/Game/SG_Objects.SG_Objects_C|SetPickedUpCoins _assg_objects (Variables|Default|GetAlreadyCollectedObjects)) ; the save game matches what the game instance has
  (bind _returnvalue_5 (Game|GetCurrentLevelName true))
  (SaveGame|SaveGametoSlot _assg_objects _returnvalue_5)
  (Development|PrintString "Save Successful"))